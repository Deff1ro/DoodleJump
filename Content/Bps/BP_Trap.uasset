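; BP_Trap is a one-shot trap actor that catches the player's doodle character when it hits the trap's box.
; The Box hit event filters for the player pawn and runs once, playing the trap animation on the skeletal mesh.
; It then calls FreezeCharacter on BP_DoodleCharacter, passing itself as the attach actor, and destroys itself shortly after the freeze duration ends.
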(event `self.Box.OnComponentBeginOverlap`
  (params (OverlappedComponent :type "PrimitiveComponent Object Reference") (OtherActor :type "Actor Object Reference") (OtherComp :type "PrimitiveComponent Object Reference") (OtherBodyIndex :type Integer) (bFromSweep :type Boolean) (SweepResult :type "HitResult Structure (by ref)")))

(event `self.Box.OnComponentHit`
  (params (HitComponent :type "PrimitiveComponent Object Reference") (OtherActor :type "Actor Object Reference") (OtherComp :type "PrimitiveComponent Object Reference") (NormalImpulse :type "Vector Structure") (Hit :type "HitResult Structure (by ref)"))
  (if (== OtherActor (`GameplayStatics.GetPlayerPawn` 0))
    (`/Engine/EditorBlueprintResources/StandardMacros.DoOnce` false
      (:`Completed`
        (`SkeletalMeshComponent.PlayAnimation` (`self.SkeletalMesh`) "/Game/DoodleJumpAssets/Platforms/Trap/Trap_Anim.Trap_Anim" false)
        (bind _asbp_doodle_character (cast `/Game/Bps/BP_DoodleCharacter` OtherActor))
        (`DoodleCharacter.FreezeCharacter` _asbp_doodle_character 5.0 self)
        (`KismetSystemLibrary.Delay` 6.0)
        (`self.K2_DestroyActor`)))))

(fn `UserConstructionScript`)
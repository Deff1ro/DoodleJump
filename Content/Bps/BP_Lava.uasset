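; BP_Lava is a rising lava hazard that moves steadily upward every frame through a local Z offset scaled by delta time.
; When its Cube component overlaps the BP_DoodleCharacter, it ends play by adding the BP_MainMenu widget to the viewport.
; It then shows the mouse cursor, switches to UI-only input and pauses the game, alongside a leftover "Hello" debug print.
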(event `self.ReceiveBeginPlay`)

(event `self.ReceiveTick`
  (params (DeltaSeconds :type "Float (single-precision)"))
  (`self.K2_AddActorLocalOffset` (`KismetMathLibrary.MakeVector` 0.0 0.0 (* DeltaSeconds 50.0))))

(event `self.Cube.OnComponentBeginOverlap`
  (params (OverlappedComponent :type "PrimitiveComponent Object Reference") (OtherActor :type "Actor Object Reference") (OtherComp :type "PrimitiveComponent Object Reference") (OtherBodyIndex :type Integer) (bFromSweep :type Boolean) (SweepResult :type "HitResult Structure (by ref)"))
  (bind _returnvalue (`GameplayStatics.GetPlayerController` 0))
  (cast `/Game/Bps/BP_DoodleCharacter` OtherActor)
  (`KismetSystemLibrary.PrintString` "Hello")
  (bind _returnvalue_2 (`|CreateWidget` "/Game/Bps/BP_MainMenu.BP_MainMenu_C"))
  (`UserWidget.AddToViewport` _returnvalue_2 0)
  (set `PlayerController.bShowMouseCursor` true _returnvalue)
  (`WidgetBlueprintLibrary.SetInputMode_UIOnlyEx` _returnvalue _returnvalue_2)
  (`GameplayStatics.SetGamePaused` true))

(fn `UserConstructionScript`)